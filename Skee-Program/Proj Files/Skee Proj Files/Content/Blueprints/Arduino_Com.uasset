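; Arduino_Com is a Blueprint that sends commands to an Arduino over a serial connection to query the board and drive a solenoid.
; It opens a fixed COM port on BeginPlay, keeps the port reference, and closes it on EndPlay.
; The Communicate event checks that the port is valid, then maps each enum command to a single-character code printed to the port.
; It only writes and never reads replies.
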(event Custom|Communicate
  (params (Communicate :type ArduinoSignal%20Enum :default "NewEnumerator0"))
  (bind _arduinoport (Variables|Default|GetArduinoPort))
  (if (Utilities|IsValid (Variables|Default|GetArduinoPort))
    (switch Utilities|FlowControl|Switch|SwitchonArduinoSignal Communicate
      (:NewEnumerator0
        (Class|Serial|Print _arduinoport "b"))
      (:NewEnumerator3
        (Class|Serial|Print _arduinoport "m"))
      (:NewEnumerator2
        (Class|Serial|Print _arduinoport "c"))
      (:NewEnumerator1
        (Class|Serial|Print _arduinoport "x")))))

(event EventBeginPlay
  (bind _returnvalue (Class|Serial|OpenComPort 3 9600))
  (Variables|Default|SetArduinoPort _returnvalue))

(event EventEndPlay
  (params (EndPlayReason :type EEndPlayReason%20Enum :default "Destroyed"))
  (Class|Serial|Close (Variables|Default|GetArduinoPort)))

(fn ConstructionScript)